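; Primal Elementalist is a boss actor that takes damage and can be killed.
; AnyDamage subtracts incoming damage from BossHealth and destroys the actor once health reaches zero or below.
; A basicAttack function applies point damage to CurrentTarget, but its only call in the event graph is unconnected and never runs.
; The construction script only calls its parent.
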(event Game|Damage|EventAnyDamage
  (params (Damage :type Float%20%28single-precision%29) (DamageType :type Damage%20Type%20Object%20Reference) (InstigatedBy :type Controller%20Object%20Reference) (DamageCauser :type Actor%20Object%20Reference))
  (bind _output_get (Variables|Default|SetbossHealth (- (Variables|Default|GetbossHealth) Damage)))
  (if (<= _output_get 0.0)
    (Actor|DestroyActor)))

(event Input|MouseEvents|LeftMouseButton
  (params (Key :type Key%20Structure)))

(fn ConstructionScript
  (|CallParentFunction))