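; Celestial is a Blueprint actor with player health that takes damage filtered through state on its Celestial_Controller.
; BeginPlay caches the player 0 controller as LinkedController.
; AnyDamage ignores hits while the controller is immune; a defended hit consumes the defense flag and scales damage by DefensiveReduction, otherwise full damage applies.
; The actor destroys itself when health reaches zero or below.
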(event EventBeginPlay
  (bind _ascelestial_controller (Utilities|Casting|CastToCelestial_Controller (Game|GetPlayerController 0)))
  (Variables|Default|SetlinkedController _ascelestial_controller))

(event Game|Damage|EventAnyDamage
  (params (Damage :type Float%20%28single-precision%29) (DamageType :type Damage%20Type%20Object%20Reference) (InstigatedBy :type Controller%20Object%20Reference) (DamageCauser :type Actor%20Object%20Reference))
  (bind _linkedcontroller (Variables|Default|GetlinkedController))
  (if (not (Variables|/Game/Blueprints/Celestial/Celestial_Controller.Celestial_Controller_C|GetisImmune _linkedcontroller))
    (if (Variables|/Game/Blueprints/Celestial/Celestial_Controller.Celestial_Controller_C|GetisDefended _linkedcontroller)
      (Utilities|FlowControl|Sequence
        (:then_0
          (Variables|/Game/Blueprints/Celestial/Celestial_Controller.Celestial_Controller_C|SetisDefended (Variables|Default|GetlinkedController) false))
        (:then_1
          (Variables|Default|SetplayerHealth (- (Variables|Default|GetplayerHealth) (* Damage (Variables|/Game/Blueprints/Celestial/Celestial_Controller.Celestial_Controller_C|GetdefensiveReduction _linkedcontroller))))
          (if (<= (Variables|Default|GetplayerHealth) 0.0) :!label _label
            (Actor|DestroyActor))))
      (else
        (Variables|Default|SetplayerHealth (- (Variables|Default|GetplayerHealth) Damage))
        (goto _label)))))

(fn ConstructionScript
  (|CallParentFunction))