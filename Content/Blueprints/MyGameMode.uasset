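; Game mode that respawns the player's Celestial character after it is destroyed.
; On BeginPlay it binds to the player character's OnDestroyed event.
; When that fires, it waits a respawn delay, spawns a new Celestial at a stored transform, stores it on the Celestial_Controller and possesses it.
; It then calls Respawn to bind the destroyed event on the new pawn, repeating the cycle.
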(event Custom|OnDestroyed_Event_0
  (params (DestroyedActor :type Actor%20Object%20Reference))
  (bind _returnvalue (Game|GetPlayerController 0))
  (Utilities|FlowControl|Delay (Variables|Default|GetrespawnTimer))
  (bind _returnvalue_2 (Game|SpawnActorfromClass "/Game/Blueprints/Celestial/Celestial.Celestial_C" (Variables|Default|GetSpawn%20Transform) "Undefined" 0 0))
  (bind _ascelestial_controller (Utilities|Casting|CastToCelestial_Controller _returnvalue))
  (Variables|/Game/Blueprints/Celestial/Celestial_Controller.Celestial_Controller_C|SetcurrentPawn _ascelestial_controller _returnvalue_2)
  (Pawn|Possess _returnvalue _returnvalue_2)
  (CallFunction|Respawn))

(event Custom|Respawn
  (bind _ascelestial (Utilities|Casting|CastToCelestial (Game|GetPlayerCharacter 0)))
  (Game|AssignOnDestroyed _ascelestial (delegate Custom|OnDestroyed_Event_0)))

(event EventBeginPlay
  (bind _ascelestial (Utilities|Casting|CastToCelestial (Game|GetPlayerCharacter 0)))
  (Game|AssignOnDestroyed _ascelestial (delegate Custom|OnDestroyed_Event_0)))

(fn ConstructionScript)